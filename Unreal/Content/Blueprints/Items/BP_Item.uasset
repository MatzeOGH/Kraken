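; BP_Item is an item actor, apparently a base class, that drifts toward the world origin at constant speed with its height pinned.
; Its Reg event calls UpdateSaveGame, sends itself to BP_HUD's Message, then destroys the actor.
; UpdateSaveGame is an empty hook, while GetSaveGame loads the BP_Savegame slot or creates and saves a new one when none is valid.
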(event Custom|Reg
  (CallFunction|UpdateSaveGame)
  (bind _asbp_hud (Utilities|Casting|CastToBP_HUD (HUD|GetHUD (Game|GetPlayerController 0))))
  (Default|Message _asbp_hud self)
  (Actor|DestroyActor))

(event EventTick
  (params (DeltaSeconds :type Float%20%28single-precision%29))
  (bind _returnvalue (Transformation|GetActorLocation))
  (bind _returnvalue_2 (* 5e+01 DeltaSeconds))
  (bind _returnvalue_3 (- "0,0.000000, 0" _returnvalue))
  (bind _returnvalue_4 (Math|Vector|Normalize _returnvalue_3))
  (bind _returnvalue_5 (* _returnvalue_4 _returnvalue_2))
  (bind _returnvalue_6 (+ _returnvalue _returnvalue_5))
  (Transformation|SetActorLocation (Math|Vector|MakeVector (.x _returnvalue_6) (.y _returnvalue_6) 1.0) false))

(fn ConstructionScript)

(fn UpdateSaveGame)

(fn GetSaveGame
  (bind _returnvalue (SaveGame|LoadGamefromSlot "Savegame"))
  (bind _asbp_savegame (Utilities|Casting|CastToBP_Savegame _returnvalue)
    (:then
      (Utilities|IsValid _asbp_savegame
        (:Is%20Valid
          (LocalVariables|Setreturn _asbp_savegame))
        (:Is%20Not%20Valid
          (bind _returnvalue_2 (SaveGame|CreateSaveGameObject "/Game/Blueprints/BP_Savegame.BP_Savegame_C" :!label _label))
          (SaveGame|SaveGametoSlot _returnvalue_2 "Savegame")
          (bind _asbp_savegame_2 (Utilities|Casting|CastToBP_Savegame _returnvalue_2)
            (:then
              (LocalVariables|Setreturn _asbp_savegame_2))
            (:CastFailed
              _)))))
    (:CastFailed
      (goto _label)))
  (return (LocalVariables|Getreturn)))