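; Multiplayer game mode Blueprint that decides when the match ends based on the Kraken's state.
; Its CheckforGameOver event casts player 0's pawn to BP_Kraken and, if all four tentacle health values are at or below zero, calls GameOver with false.
; BeginPlay, Tick and the construction script hold no custom logic, so the check runs only when the event is called.
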(event `self.ReceiveBeginPlay`)

(event `self.ReceiveTick`
  (params (DeltaSeconds :type "Float (single-precision)")))

(event `self.CheckForGameOver`
  (bind _asbp_kraken (cast `/Game/Blueprints/BP_Kraken` (`GameplayStatics.GetPlayerPawn` 0)))
  (if (and (<= (`/Game/Blueprints/BP_Kraken.Tentacle1Health` _asbp_kraken) 0.0) (<= (`/Game/Blueprints/BP_Kraken.Tentacle2Health` _asbp_kraken) 0.0) (<= (`/Game/Blueprints/BP_Kraken.Tentacle3Health` _asbp_kraken) 0.0) (<= (`/Game/Blueprints/BP_Kraken.Tentacle4Health` _asbp_kraken) 0.0))
    (`self.GameOver` false)))

(fn `UserConstructionScript`
  (`parent.UserConstructionScript`))