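; Game mode for a Kraken ship-sinking game, managing ship spawns, scoring and game over.
; A looping timer has random BP_Path actors spawn ships below a cap, which rises every five kills.
; ShipSank adds tentacle score to the GameState and spawns a ship at a random TargetPoint, facing world origin.
; CheckForGameOver ends in defeat when any tentacle dies, updating the save object's high score without writing it to the slot.
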(event Custom|SpawnShip
  (bind _outactors (Actor|GetAllActorsOfClass "/Script/Engine.TargetPoint"))
  (Utilities|IsValid (Utilities|Array|Get(acopy) _outactors (Math|Random|RandomIntegerinRange 0 (- (Utilities|Array|Length _outactors) 1)))
    (:Is%20Valid
      (Game|SpawnActorfromClass "/Game/Blueprints/BP_Ship.BP_Ship_C" (Math|Transform|MakeTransform (Transformation|GetActorLocation (Utilities|Array|Get(acopy) _outactors (Math|Random|RandomIntegerinRange 0 (- (Utilities|Array|Length _outactors) 1)))) (Math|Rotator|MakeRotfromX (- "0, 0, 0" (Transformation|GetActorLocation (Utilities|Array|Get(acopy) _outactors (Math|Random|RandomIntegerinRange 0 (- (Utilities|Array|Length _outactors) 1))))))) false 0 0))))

(event Custom|TickGameMode
  (bind _outactors (Actor|GetAllActorsOfClass "/Game/Blueprints/BP_Ship.BP_Ship_C"))
  (if (< (Utilities|Array|Length _outactors) (Variables|Default|GetMaxShips))
    (bind _outactors_2 (Actor|GetAllActorsOfClass "/Game/Blueprints/BP_Path.BP_Path_C" :!label _label))
    (Utilities|IsValid (Variables|/Game/Blueprints/BP_Path.BP_Path_C|GetShip (Utilities|Array|Get(acopy) _outactors_2 (Math|Random|RandomIntegerinRange 0 (- (Utilities|Array|Length _outactors_2) 1))))
      (:Is%20Valid
        (goto _label))
      (:Is%20Not%20Valid
        (Default|SpawnShip (Utilities|Array|Get(acopy) _outactors_2 (Math|Random|RandomIntegerinRange 0 (- (Utilities|Array|Length _outactors_2) 1))))))))

(event Custom|ShipSank
  (params (Tentacle :type Integer) (Score :type Integer))
  (bind _asbp_game_state (Utilities|Casting|CastToBP_GameState (Game|GetGameState)))
  (Default|AddScore _asbp_game_state Tentacle Score)
  (CallFunction|SpawnShip))

(event Custom|IncreaseShipCount
  (Variables|Default|SetMaxShips (+ (Variables|Default|GetMaxShips) 1)))

(event Custom|Kill
  (bind _output_get (Variables|Default|SetKills (+ (Variables|Default|GetKills) 1)))
  (if (>= _output_get 5)
    (Variables|Default|SetKills 0)
    (CallFunction|IncreaseShipCount)))

(event Custom|GameOver
  (params (bWon :type Boolean))
  (bind _asbp_hud (Utilities|Casting|CastToBP_HUD (HUD|GetHUD (Game|GetPlayerController 0))))
  (Default|DisplayGameoverScreen _asbp_hud bWon)
  (Game|SetGamePaused true))

(event EventBeginPlay
  (Utilities|Time|SetTimerbyFunctionName self "TickGameMode" 3.0 true))

(fn ConstructionScript)

(fn CheckforGameOver
  (bind _returnvalue (Game|GetGameState))
  (bind _asbp_game_state (Utilities|Casting|CastToBP_GameState _returnvalue))
  (bind _return (Default|GetSPScore _asbp_game_state))
  (bind _asbp_kraken (Utilities|Casting|CastToBP_Kraken (Game|Player|GetPlayerPawn 0)))
  (if (Math|Boolean|ORBoolean (<= (Variables|/Game/Blueprints/BP_Kraken.BP_Kraken_C|GetTentacle1Health _asbp_kraken) 0.0) (<= (Variables|/Game/Blueprints/BP_Kraken.BP_Kraken_C|GetTentacle2Health _asbp_kraken) 0.0) (<= (Variables|/Game/Blueprints/BP_Kraken.BP_Kraken_C|GetTentacle3Health _asbp_kraken) 0.0) (<= (Variables|/Game/Blueprints/BP_Kraken.BP_Kraken_C|GetTentacle4Health _asbp_kraken) 0.0))
    (bind _returnvalue_2 (SaveGame|LoadGamefromSlot "Savegame"))
    (bind _asbp_savegame (Utilities|Casting|CastToBP_Savegame _returnvalue_2)
      (:then
        (Utilities|IsValid _asbp_savegame
          (:Is%20Valid
            (LocalVariables|SetSaveGame _asbp_savegame))))
      (:CastFailed
        (bind _returnvalue_3 (SaveGame|CreateSaveGameObject "/Game/Blueprints/BP_Savegame.BP_Savegame_C"))
        (bind _asbp_savegame_2 (Utilities|Casting|CastToBP_Savegame _returnvalue_3))
        (LocalVariables|SetSaveGame _asbp_savegame_2)))
    (if (> _return (Variables|/Game/Blueprints/BP_Savegame.BP_Savegame_C|GetHighScore (LocalVariables|GetSaveGame)))
      (Variables|/Game/Blueprints/BP_Savegame.BP_Savegame_C|SetHighScore (LocalVariables|GetSaveGame) _return))
    (CallFunction|GameOver false)))