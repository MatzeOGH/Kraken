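; Game state Blueprint that tracks a separate score for each of four tentacles.
; The AddScore event switches on the tentacle number and adds the given score to that tentacle's running total.
; GetSPScore returns the sum of all four tentacle scores as one combined score.
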(event `AddScore`
  (params (Tentacle :type Integer) (Score :type Integer))
  (switch `int` Tentacle
    (:`1`
      (set `self.Tentacle1Score` (+ (`self.Tentacle1Score`) Score)))
    (:`2`
      (set `self.Tentacle2Score` (+ (`self.Tentacle2Score`) Score)))
    (:`3`
      (set `self.Tentacle3Score` (+ (`self.Tentacle3Score`) Score)))
    (:`4`
      (set `self.Tentacle4Score` (+ (`self.Tentacle4Score`) Score)))))

(fn `GetSPScore`
  (returns (Return :type Integer))
  (return (+ (`self.Tentacle1Score`) (`self.Tentacle2Score`) (`self.Tentacle3Score`) (`self.Tentacle4Score`))))

(fn `UserConstructionScript`)