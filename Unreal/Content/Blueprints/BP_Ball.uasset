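; BP_Ball is a cannonball projectile that damages the Kraken on hit.
; On BeginPlay a timeline drives the sprite's uniform scale over the ball's lifetime, then destroys the actor without an explosion.
; Kraken hits apply point damage, then share the Explode event's path of spawning a small explosion and destroying the ball.
; Other hits do nothing, and an island-hit branch is left unconnected.
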(event `self.ReceiveBeginPlay`
  (bind (_direction _scale) (`Timeline|Timeline_0`)
    (:`Update`
      (`SceneComponent.SetRelativeScale3D` (`self.cannonball_Sprite`) (`KismetMathLibrary.MakeVector` _scale _scale _scale)))
    (:`Finished`
      (`self.K2_DestroyActor`))))

(event `self.ReceiveHit`
  (params (MyComp :type "PrimitiveComponent Object Reference") (Other :type "Actor Object Reference") (OtherComp :type "PrimitiveComponent Object Reference") (bSelfMoved :type Boolean) (HitLocation :type "Vector Structure") (HitNormal :type "Vector Structure") (NormalImpulse :type "Vector Structure") (Hit :type "HitResult Structure (by ref)"))
  (`|ExecutionSequence`
    (:`then_0`
      (cast `/Game/Blueprints/BP_Kraken` Other)
      (`GameplayStatics.ApplyPointDamage` Other 10.0 HitNormal Hit null null "/Script/Engine.DamageType")
      (`|SpawnActorFromClass` "/Game/Blueprints/BP_ExplosionSmall.BP_ExplosionSmall_C" (`KismetMathLibrary.MakeTransform` (`self.K2_GetActorLocation`)) :!label _label)
      (`self.K2_DestroyActor`))))

(event `self.ReceiveDestroyed`)

(event `Explode`
  (goto _label))

(fn `UserConstructionScript`)