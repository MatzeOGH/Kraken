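; BP_Kraken is a touch-controlled kraken whose four tentacles follow separate fingers and take damage individually.
; On BeginPlay it gives each ABP_Tentacle anim instance a start location and anchor, and sets per-bone physics simulation.
; Tick moves held tentacles to the offset finger hit point at zero height and eases released ones toward their start.
; Point damage decrements the hit tentacle's health and has BP_Gamemode check for game over.
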(event `self.ReceiveBeginPlay`
  (`self.InitTentacle` (`self.Tentacle1`) "Tentacle_Joint15" (`self.T1Start`) (-1000.0 0.0 0.0))
  (`self.InitTentacle` (`self.Tentacle2`) "Tentacle_Joint15" (`self.T2Start`) (1000.0 0.0 0.0))
  (`self.InitTentacle` (`self.Tentacle3`) "Tentacle_Joint15" (`self.T3Start`) (0.0 -1000.0 0.0))
  (`self.InitTentacle` (`self.Tentacle4`) "Tentacle_Joint15" (`self.T4Start`) (0.0 1000.0 0.0)))

(event `self.Tentacle1.OnInputTouchBegin`
  (params (FingerIndex :type "ETouchIndex Enum" :default "Touch1") (TouchedComponent :type "PrimitiveComponent Object Reference"))
  ;[1 1 1] Comment
  (if (`.ReturnValue` (`PlayerController.GetHitResultUnderFingerForObjects` (`GameplayStatics.GetPlayerController` 0) FingerIndex (`|MakeArray` "ObjectTypeQuery2" :!type "EObjectTypeQuery Enum") true))
    (set `self.bTentacle1` true)
    (set `self.Tentacle1Touch` FingerIndex)))

(event `self.Tentacle2.OnInputTouchBegin`
  (params (FingerIndex :type "ETouchIndex Enum" :default "Touch1") (TouchedComponent :type "PrimitiveComponent Object Reference"))
  (if (`.ReturnValue` (`PlayerController.GetHitResultUnderFingerForObjects` (`GameplayStatics.GetPlayerController` 0) FingerIndex (`|MakeArray` "ObjectTypeQuery2" :!type "EObjectTypeQuery Enum") true))
    (set `self.bTentacle2` true)
    (set `self.Tentacle2Touch` FingerIndex)))

(event `self.Tentacle3.OnInputTouchBegin`
  (params (FingerIndex :type "ETouchIndex Enum" :default "Touch1") (TouchedComponent :type "PrimitiveComponent Object Reference"))
  (if (`.ReturnValue` (`PlayerController.GetHitResultUnderFingerForObjects` (`GameplayStatics.GetPlayerController` 0) FingerIndex (`|MakeArray` "ObjectTypeQuery2" :!type "EObjectTypeQuery Enum") true))
    (set `self.bTentacle3` true)
    (set `self.Tentacle3Touch` FingerIndex)))

(event `self.Tentacle4.OnInputTouchBegin`
  (params (FingerIndex :type "ETouchIndex Enum" :default "Touch1") (TouchedComponent :type "PrimitiveComponent Object Reference"))
  (if (`.ReturnValue` (`PlayerController.GetHitResultUnderFingerForObjects` (`GameplayStatics.GetPlayerController` 0) FingerIndex (`|MakeArray` "ObjectTypeQuery2" :!type "EObjectTypeQuery Enum") true))
    (set `self.bTentacle4` true)
    (set `self.Tentacle4Touch` FingerIndex)))

(event `self.Tentacle2.OnInputTouchEnd`
  (params (FingerIndex :type "ETouchIndex Enum" :default "Touch1") (TouchedComponent :type "PrimitiveComponent Object Reference"))
  (set `self.bTentacle2` false))

(event `self.Tentacle3.OnInputTouchEnd`
  (params (FingerIndex :type "ETouchIndex Enum" :default "Touch1") (TouchedComponent :type "PrimitiveComponent Object Reference"))
  (set `self.bTentacle3` false))

(event `self.Tentacle1.OnInputTouchEnd`
  (params (FingerIndex :type "ETouchIndex Enum" :default "Touch1") (TouchedComponent :type "PrimitiveComponent Object Reference"))
  ;[1 1 1] Comment
  (set `self.bTentacle1` false))

(event `self.Tentacle4.OnInputTouchEnd`
  (params (FingerIndex :type "ETouchIndex Enum" :default "Touch1") (TouchedComponent :type "PrimitiveComponent Object Reference"))
  (set `self.bTentacle4` false))

(event `self.ReceivePointDamage`
  (params (Damage :type "Float (single-precision)") (DamageType :type "DamageType Object Reference") (HitLocation :type "Vector Structure") (HitNormal :type "Vector Structure") (HitComponent :type "PrimitiveComponent Object Reference") (BoneName :type Name) (ShotFromDirection :type "Vector Structure") (InstigatedBy :type "Controller Object Reference") (DamageCauser :type "Actor Object Reference"))
  (switch `string` (`KismetSystemLibrary.GetObjectName` HitComponent)
    (:`Tentacle1`
      (set `self.Tentacle1Health` (- (`self.Tentacle1Health`) 1.0)))
    (:`Tentacle2`
      (set `self.Tentacle2Health` (- (`self.Tentacle2Health`) 1.0)))
    (:`Tentacle3`
      (set `self.Tentacle3Health` (- (`self.Tentacle3Health`) 1.0)))
    (:`Tentacle4`
      (set `self.Tentacle4Health` (- (`self.Tentacle4Health`) 1.0))))
  (bind _asbp_gamemode (cast `/Game/Blueprints/BP_Gamemode` (`GameplayStatics.GetGameMode`)))
  (`/Game/Blueprints/BP_Gamemode.CheckForGameOver` _asbp_gamemode))

(event `self.ReceiveTick`
  (params (DeltaSeconds :type "Float (single-precision)"))
  (`|ExecutionSequence`
    (:`then_0`
      (`self.UpdateTentacle` (`self.bTentacle1`) (`self.Tentacle1Touch`) (`self.Tentacle1`) (50.0 0.0 0.0) (`self.T1Start`)))
    (:`then_1`
      (`self.UpdateTentacle` (`self.bTentacle2`) (`self.Tentacle2Touch`) (`self.Tentacle2`) (-50.0 0.0 0.0) (`self.T2Start`)))
    (:`then_2`
      (`self.UpdateTentacle` (`self.bTentacle3`) (`self.Tentacle3Touch`) (`self.Tentacle3`) (0.0 50.0 0.0) (`self.T3Start`)))
    (:`then_3`
      (`self.UpdateTentacle` (`self.bTentacle4`) (`self.Tentacle4Touch`) (`self.Tentacle4`) (0.0 -50.0 0.0) (`self.T4Start`)))))

(fn `InitTentacle`
  (params (self2 :type "SkeletalMeshComponent Object Reference") (InBoneName :type "Name (by ref)") (Location :type "Vector Structure") (Anker :type "Vector Structure"))
  (bind _asabp_tentacle (cast `/Game/Kraken/ABP_Tentacle` (`SkeletalMeshComponent.GetAnimInstance` self2))
    (:`then`
      (`/Game/Kraken/ABP_Tentacle.SetLocation` _asabp_tentacle Location)
      (set `/Game/Kraken/ABP_Tentacle.Anker` Anker _asabp_tentacle)
      (`SkeletalMeshComponent.SetAllBodiesBelowSimulatePhysics` self2 InBoneName true)
      (`SkeletalMeshComponent.SetAllBodiesBelowSimulatePhysics` self2 "Tentacle_Joint2" false))
    (:`CastFailed`
      _))
  (return))

(fn `UpdateTentacle`
  (params (Condition :type Boolean) (FingerIndex :type "ETouchIndex Enum") (Target :type "SkeletalMeshComponent Object Reference") (Offset :type "Vector Structure") (B :type "Vector Structure"))
  (bind (_hitresult _returnvalue) (`PlayerController.GetHitResultUnderFingerForObjects` (`GameplayStatics.GetPlayerController` 0) FingerIndex (`|MakeArray` "ObjectTypeQuery2" :!type "EObjectTypeQuery Enum") true))
  (bind (_returnvalue_x _returnvalue_y) (`KismetMathLibrary.BreakVector` (+ (`.Location` (`GameplayStatics.BreakHitResult` _hitresult)) Offset)))
  (if Condition
    (if _returnvalue
      (bind _asabp_tentacle (cast `/Game/Kraken/ABP_Tentacle` (`SkeletalMeshComponent.GetAnimInstance` Target))
        (:`then`
          (`/Game/Kraken/ABP_Tentacle.SetLocation` _asabp_tentacle (`KismetMathLibrary.MakeVector` _returnvalue_x _returnvalue_y)))
        (:`CastFailed`
          _)))
    (else
      (bind _asabp_tentacle_2 (cast `/Game/Kraken/ABP_Tentacle` (`SkeletalMeshComponent.GetAnimInstance` Target))
        (:`then`
          (`/Game/Kraken/ABP_Tentacle.SetLocation` _asabp_tentacle_2 (`KismetMathLibrary.VLerp` (`SceneComponent.GetSocketLocation` Target "Tentacle_Joint16") B (* (`GameplayStatics.GetWorldDeltaSeconds`) 2.0))))
        (:`CastFailed`
          _))))
  (return))

(fn `UserConstructionScript`)