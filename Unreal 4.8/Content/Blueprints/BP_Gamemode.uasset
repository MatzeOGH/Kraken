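; BP_Gamemode is the game mode that handles ship spawning, scoring and game over.
; SpawnShip creates a BP_Ship at a random TargetPoint in the level, rotated to face the world origin.
; ShipSank passes the tentacle and score to BP_GameState, then spawns another ship.
; GameOver tells the first player's BP_HUD to show the game-over screen with the win result.
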(event `GameOver`
  (params (bWon :type Boolean))
  (bind _asbp_hud (cast `/Game/Blueprints/BP_HUD` (`PlayerController.GetHUD` (`GameplayStatics.GetPlayerController` 0))))
  (`/Game/Blueprints/BP_HUD.Display Gameover Screen` _asbp_hud bWon))

(event `SpawnShip`
  (bind _outactors (`GameplayStatics.GetAllActorsOfClass` "/Script/Engine.TargetPoint"))
  (bind _item (`KismetArrayLibrary.Array_Get` _outactors (`KismetMathLibrary.RandomIntegerInRange` 0 (- (`KismetArrayLibrary.Array_Length` _outactors) 1))))
  (`/Engine/EditorBlueprintResources/StandardMacros.IsValid` _item
    (:`Is Valid`
      (bind _returnvalue (`self.K2_GetActorLocation` _item))
      (`|SpawnActorFromClass` "/Game/Blueprints/BP_Ship.BP_Ship_C" (`KismetMathLibrary.MakeTransform` _returnvalue (`KismetMathLibrary.MakeRotFromX` (- (0.0 0.0 0.0) _returnvalue)))))))

(event `ShipSank`
  (params (Tentacle :type Integer) (Score :type Integer))
  (bind _asbp_game_state (cast `/Game/Blueprints/BP_GameState` (`GameplayStatics.GetGameState`)))
  (`/Game/Blueprints/BP_GameState.AddScore` _asbp_game_state Tentacle Score)
  (`self.SpawnShip`))

(fn `UserConstructionScript`)