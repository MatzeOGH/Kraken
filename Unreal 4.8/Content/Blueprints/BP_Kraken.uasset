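; Kraken Blueprint with a tentacle that the player drags by touch.
; BeginPlay enables physics simulation on the bones below Tentacle_Joint15 and passes a start location to the tentacle's ABP_Tentacle anim instance.
; Touching Tentacle1 stores the finger index, and Tick traces WorldDynamic objects under that finger, sending the hit X/Y at zero Z to the anim instance.
; Releasing stops the drag and prints a debug string.
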(event `self.ReceiveBeginPlay`
  (`SkeletalMeshComponent.SetAllBodiesBelowSimulatePhysics` (`self.Tentacle1`) "Tentacle_Joint15" true)
  (bind _asabp_tentacle (cast `/Game/Kraken/ABP_Tentacle` (`SkeletalMeshComponent.GetAnimInstance` (`self.Tentacle1`))))
  (`/Game/Kraken/ABP_Tentacle.SetLocation` _asabp_tentacle (`self.T1StartLoc`)))

(event `self.Tentacle1.OnInputTouchBegin`
  (params (FingerIndex :type "ETouchIndex Enum") (TouchedComponent :type "PrimitiveComponent Object Reference"))
  (if (`.ReturnValue` (`PlayerController.GetHitResultUnderFingerForObjects` (`GameplayStatics.GetPlayerController` 0) FingerIndex (`|MakeArray` "ObjectTypeQuery2" :!type "EObjectTypeQuery Enum") true))
    (set `self.bMoveTentacle1` true)
    (set `self.MoveTentacel1Input` FingerIndex)))

(event `self.Tentacle1.OnInputTouchEnd`
  (params (FingerIndex :type "ETouchIndex Enum" :default "Touch1") (TouchedComponent :type "PrimitiveComponent Object Reference"))
  (set `self.bMoveTentacle1` false)
  (`KismetSystemLibrary.PrintString` "Hello"))

(event `self.ReceiveTick`
  (params (DeltaSeconds :type "Float (single-precision)"))
  (bind (_hitresult _returnvalue) (`PlayerController.GetHitResultUnderFingerForObjects` (`GameplayStatics.GetPlayerController` 0) (`self.MoveTentacel1Input`) (`|MakeArray` "ObjectTypeQuery2" :!type "EObjectTypeQuery Enum") true))
  (`|ExecutionSequence`
    (:`then_0`
      (if (`self.bMoveTentacle1`)
        (if _returnvalue
          (bind _asabp_tentacle (cast `/Game/Kraken/ABP_Tentacle` (`SkeletalMeshComponent.GetAnimInstance` (`self.Tentacle1`))))
          (`/Game/Kraken/ABP_Tentacle.SetLocation` _asabp_tentacle (`KismetMathLibrary.MakeVector` (.x (`.Location` (`GameplayStatics.BreakHitResult` _hitresult))) (.y (`.Location` (`GameplayStatics.BreakHitResult` _hitresult))))))))))

(fn `UserConstructionScript`)