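; BP_Ship is a ship actor that loses health while touched and sinks when it runs out.
; Touch begin and end open and close a Tick gate that drains Health by delta time.
; On death it reports its random TentacleID and a score to BP_Gamemode's ShipSank, then destroys itself.
; Tick also draws Health and ID as debug text; SetIDColor is an unfinished stub.
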(event `self.ReceiveBeginPlay`
  ;[1 1 1] set the id for the tentacle
  (set `self.TentacleID` (`KismetMathLibrary.RandomIntegerInRange` 1 4)))

(event `self.ReceiveTick`
  (params (DeltaSeconds :type "Float (single-precision)"))
  (`|ExecutionSequence`
    (:`then_0`
      (`/Engine/EditorBlueprintResources/StandardMacros.Gate` true :!label _label
        (:`Exit`
          ;[0.3449 1 0.3587] decrease
          (set `self.Health` (- (`self.Health`) DeltaSeconds))
          ;[1 0.1176 0.4613] Did we die?
          (if (<= (`self.Health`) 0.0)
            (`self.Die`)))))
    (:`then_1`
      (`self.PrintDebug` DeltaSeconds))))

(event `self.ReceiveActorOnInputTouchBegin`
  (params (FingerIndex :type "ETouchIndex Enum" :default "Touch1"))
  (goto _label :!via `Open`))

(event `self.ReceiveActorOnInputTouchEnd`
  (params (FingerIndex :type "ETouchIndex Enum" :default "Touch1"))
  (goto _label :!via `Close`))

(event `Die`
  (bind _asbp_gamemode (cast `/Game/Blueprints/BP_Gamemode` (`GameplayStatics.GetGameMode`)))
  (`/Game/Blueprints/BP_Gamemode.ShipSank` _asbp_gamemode (`self.TentacleID`) 1)
  (`self.K2_DestroyActor`))

(fn `PrintDebug`
  (params (Duration :type "Float (double-precision)"))
  (`KismetSystemLibrary.DrawDebugString` (0.0 0.0 0.0) (`KismetStringLibrary.Concat_StrStr` "HP" (`KismetStringLibrary.Conv_DoubleToString` (`self.Health`)) "  ID:" (`KismetStringLibrary.Conv_IntToString` (`self.TentacleID`))) self (struct :`R` 1.0 :`B` 0.433233 :`A` 1.0) Duration))

(fn `SetIDColor`)

(fn `UserConstructionScript`)